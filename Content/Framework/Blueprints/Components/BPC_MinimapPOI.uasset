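; Actor component that registers its owning actor as a point of interest on the minimap.
; InitialisePOI receives the game mode, caches it along with its main HUD and minimap widget, then triggers icon creation.
; CreatePOIIcon passes the owner to the minimap widget to create the icon.
; A following exact-class check for BP_BaseQuestLocation leads to no further logic.
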(event Custom|CreatePOIIcon
  (bind _returnvalue (Components|GetOwner))
  ;[0 0.734 0.07641] Create POI Icon in the Minimap Widget
  (Default|CreatePOIIcon (Variables|Default|GetWBP%20Mini%20Map) _returnvalue)
  (if (== (Utilities|GetClass _returnvalue) "/Game/Framework/Blueprints/Quest/BP_BaseQuestLocation.BP_BaseQuestLocation_C")
    _))

(event EventInitialisePOI
  (params (ModeRef :type BP%20RPG%20Mode%20Object%20Reference))
  (bind _output_get (Variables|Default|SetGame%20Mode%20Ref ModeRef))
  (bind _output_get_2 (Variables|Default|SetMainUIHUD (Variables|/Game/Framework/Blueprints/Modes/BP_RPGMode.BP_RPGMode_C|GetMainHUD _output_get)))
  ;[0 0.734 0.07641] Save Minimap Widget Reference
  (Variables|Default|SetWBP%20Mini%20Map (Variables|/Game/StudentWork/UI/WBP_MainUIHUD.WBP_MainUIHUD_C|GetWBP_MiniMap _output_get_2))
  (CallFunction|CreatePOIIcon))