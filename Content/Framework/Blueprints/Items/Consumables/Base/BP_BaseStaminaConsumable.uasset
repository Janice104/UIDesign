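; Base consumable item Blueprint that restores a character's stamina when consumed.
; Its ConsumeEffect compares CurrentStamina to MaxStamina on the consuming character's BPCAttributes component and, if below max, adds StaminaUpdateAmount through ModifyStamina.
; It returns true when stamina is applied and false when already full, while the event graph and construction script add no logic of their own.
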(event EventBeginPlay
  (|CallParentFunction) ; This node is disabled and will not be called.\nDrag off pins to build functionality.
)

(event Collision|EventActorBeginOverlap
  (params (OtherActor :type Actor%20Object%20Reference))
  (|CallParentFunction OtherActor) ; This node is disabled and will not be called.\nDrag off pins to build functionality.
)

(event EventTick
  (params (DeltaSeconds :type Float%20%28single-precision%29))
  (|CallParentFunction DeltaSeconds) ; This node is disabled and will not be called.\nDrag off pins to build functionality.
)

(fn ConstructionScript
  (|CallParentFunction))

(fn ConsumeEffect
  (params (ConsumingCharacter :type BP%20Base%20Character%20Object%20Reference))
  (bind _bpc_attributes (Variables|/Game/Framework/Blueprints/Characters/BP_BaseCharacter.BP_BaseCharacter_C|GetBPC_Attributes ConsumingCharacter))
  (bind _gameplayattributes (Variables|/Game/Framework/Blueprints/Components/BPC_Attributes.BPC_Attributes_C|GetGameplayAttributes _bpc_attributes))
  (bind (_currentstamina _maxstamina) (Utilities|Struct|BreakStruct_GameplayAttributes _gameplayattributes))
  (if (< _currentstamina _maxstamina)
    (Default|ModifyStamina _bpc_attributes true (Variables|ConsumeEffect|GetStaminaUpdateAmount))
    (return true)
    (else
      (return false))))